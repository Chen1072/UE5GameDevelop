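; BP_LaserBeam is a weapon laser that renders a colored beam with an impact effect and point light.
; BeginPlay applies LaserColor to the beam, impact effect and light.
; Each Tick, a Visibility line trace runs forward from the root over Range, feeding the impact-point distance into the beam's "Beam End" X parameter.
; The impact effect and light move to the hit location and show only on a blocking hit.
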(event `self.ReceiveBeginPlay`
  (`FXSystemComponent.SetColorParameter` (`self.LaserBeam`) "Color" (`self.LaserColor`))
  (`FXSystemComponent.SetColorParameter` (`self.LaserImpact`) "Color" (`self.LaserColor`))
  (`LightComponent.SetLightColor` (`self.PointLight`) (`self.LaserColor`) true))

(event `self.ReceiveTick`
  (params (DeltaSeconds :type "Float (single-precision)"))
  (bind _defaultsceneroot (`self.DefaultSceneRoot`))
  (bind _laserimpact (`self.LaserImpact`))
  (bind _returnvalue (`SceneComponent.K2_GetComponentLocation` _defaultsceneroot))
  (bind _outhit (`KismetSystemLibrary.LineTraceSingle` _returnvalue (+ _returnvalue (* (`SceneComponent.GetForwardVector` _defaultsceneroot) (`self.Range`))) "TraceTypeQuery1"))
  (bind (_bblockinghit _binitialoverlap _time _distance _location _impactpoint) (`GameplayStatics.BreakHitResult` _outhit))
  (set `self.Blocking Hit` _bblockinghit)
  (set `self.Hit Location` _location)
  (`FXSystemComponent.SetVectorParameter` (`self.LaserBeam`) "Beam End" (`KismetMathLibrary.MakeVector` (`KismetMathLibrary.Vector_Distance` (`SceneComponent.K2_GetComponentLocation` (`self.DefaultSceneRoot`)) _impactpoint)))
  (`SceneComponent.SetVisibility` _laserimpact (`self.Blocking Hit`) false)
  (`SceneComponent.SetVisibility` (`self.PointLight`) (`self.Blocking Hit`) false)
  (`SceneComponent.K2_SetWorldLocation` _laserimpact (`self.Hit Location`) false false)
  (`SceneComponent.K2_SetWorldLocation` (`self.PointLight`) (`self.Hit Location`) false false))

(fn `UserConstructionScript`)