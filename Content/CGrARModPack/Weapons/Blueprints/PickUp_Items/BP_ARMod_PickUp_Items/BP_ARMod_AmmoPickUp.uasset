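; Interactable ammo pickup that refills the reserve ammo of the player's current weapon when it matches one hardcoded gun type and caliber.
; On interaction it reads the weapon's pickup pool size, checks caliber, and prints a message for a mismatch or full ammo.
; Otherwise it plays pickup sounds, sets AmmoMax to the pool value or the sum, and destroys itself.
; The pool-value branch also auto-reloads an empty magazine.
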(event `/Game/CGrARModPack/Weapons/Blueprints/PickUp_Master/Interfaces/BPI_Interaction.OnInteracted`
  (params (`Player 0` :type "/Game/CGrARModPack/FPS_Arms/Bluprints/BP_FPS_Arms Object Reference"))
  (bind _currentweapon (`/Game/CGrARModPack/FPS_Arms/Bluprints/BP_FPS_Arms.CurrentWeapon` `Player 0`))
  (bind _currentweapon_2 (`/Game/CGrARModPack/FPS_Arms/Bluprints/BP_FPS_Arms.CurrentWeapon` `Player 0`))
  (bind _weapondata (`/Game/CGrARModPack/Weapons/Blueprints/PickUp_Master/Gun/BP_Weapon_Base.WeaponData` _currentweapon_2))
  (bind ((`AmmoMax_16_07E5E6CD4099A151EC845390F8F05DD9` _ammomax) (`PickUp_AmmoPool_153_D0047CFE4D1648399ACE53B72548269D` _pickup_ammopool)) (break `/Game/CGrARModPack/Weapons/Blueprints/PickUp_Master/Gun/BP_WeaponData_Struct` (`/Game/CGrARModPack/Weapons/Blueprints/PickUp_Master/Gun/BP_Weapon_Base.WeaponData` _currentweapon)))
  (bind _returnvalue (+ (`self.PickUpAmmo`) _ammomax))
  (`/Engine/EditorBlueprintResources/StandardMacros.IsValid` _currentweapon
    (:`Is Valid`
      (set `self.PickupAmmo` _pickup_ammopool)
      (if (`self.Caliber_Check` _currentweapon)
        (if (== _ammomax (`self.PickUpAmmo`))
          (`KismetSystemLibrary.PrintString` "Full Ammo" true true (struct :`G` 0.2 :`B` 1.0 :`A` 1.0))
          (else
            (`self.PickUpSound` `Player 0`)
            (`self.AmmoPickUpSound` `Player 0`)
            (if (>= _returnvalue (`self.PickUpAmmo`))
              (setmembers `/Game/CGrARModPack/Weapons/Blueprints/PickUp_Master/Gun/BP_WeaponData_Struct` :`StructRef` _weapondata :`Ammo Max` (`self.PickUpAmmo`))
              (`self.K2_DestroyActor`)
              (if (== (`.AmmoCurrent_20_1887021F4D4CB2E5D9F559887095BC17` (break `/Game/CGrARModPack/Weapons/Blueprints/PickUp_Master/Gun/BP_WeaponData_Struct` _weapondata)) 0)
                (`/Game/CGrARModPack/Weapons/Blueprints/PickUp_Master/Gun/BP_Weapon_Base.AutoReload` _currentweapon_2))
              (else
                (setmembers `/Game/CGrARModPack/Weapons/Blueprints/PickUp_Master/Gun/BP_WeaponData_Struct` :`StructRef` _weapondata :`Ammo Max` _returnvalue)
                (`self.K2_DestroyActor`)))))
        (else
          (`KismetSystemLibrary.PrintString` "Ammo Not Match" true true (struct :`R` 1.0 :`A` 1.0)))))))

(fn `AmmoPickUpSound`
  (params (Out_Player :type "/Game/CGrARModPack/FPS_Arms/Bluprints/BP_FPS_Arms Object Reference"))
  (`GameplayStatics.PlaySoundAtLocation` "/Game/CGrARModPack/Weapons/Audio/SC_Mag_insert_Empty_Cue.SC_Mag_insert_Empty_Cue" (`SceneComponent.K2_GetComponentLocation` (`/Game/CGrARModPack/FPS_Arms/Bluprints/BP_FPS_Arms.Arms` Out_Player)) (struct) 1.0 1.0 0.0 null null null)
  (return))

(fn `Caliber_Check`
  (params (`GunType&Caliber` :type "/Game/CGrARModPack/Weapons/Blueprints/PickUp_Master/Gun/BP_Weapon_Base Object Reference"))
  (returns (`  ` :type Boolean))
  ;[0 0 0] Index in "E_GunType_and_Caliber_Enum"
  (return (== (`.GunTypeandCaliber_147_AE58B3FF49A26D3AE1287F8D49F53418` (break `/Game/CGrARModPack/Weapons/Blueprints/PickUp_Master/Gun/BP_WeaponData_Struct` (`/Game/CGrARModPack/Weapons/Blueprints/PickUp_Master/Gun/BP_Weapon_Base.WeaponData` `GunType&Caliber`))) 3)))

(fn `UserConstructionScript`
  (`parent.UserConstructionScript`))