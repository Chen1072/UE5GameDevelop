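; Pickup actor, named for gun attachments or ammo, that shows its name when the player is nearby and offers a "Pick Up" interaction prompt.
; Tick measures the distance to player 0's pawn and shows or hides the name widget at a fixed range.
; The name widget is created lazily on first show from PickUpName and assigned to the Widget component.
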(event `ShowName`
  (bind _widget (`self.Widget`))
  (`/Engine/EditorBlueprintResources/StandardMacros.IsValid` (`self.WB_Name`)
    (:`Is Valid`
      _)
    (:`Is Not Valid`
      (bind _returnvalue (`|CreateWidget` "/Game/CGrARModPack/Weapons/Blueprints/PickUp_Master/WB_PickUp_Name.WB_PickUp_Name_C" null (`self.PickUp Name`)))
      (bind _output_get (set `self.WB_Name` _returnvalue))
      (`WidgetComponent.SetWidget` _widget _output_get)))
  (`SceneComponent.SetVisibility` _widget true false))

(event `HideName`
  (`SceneComponent.SetVisibility` (`self.Widget`) false false))

(event `self.ReceiveTick`
  (params (DeltaSeconds :type "Float (single-precision)"))
  (if (< (`KismetMathLibrary.Vector_Distance` (`self.K2_GetActorLocation` (`GameplayStatics.GetPlayerPawn` 0)) (`self.K2_GetActorLocation`)) 350.0)
    (`self.ShowName`)
    (else
      (`self.HideName`))))

(fn `Get Interaction Text`
  (returns (text :type Text))
  (return "Pick Up"))

(fn `UserConstructionScript`
  (`parent.UserConstructionScript`))