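; BP_AOE_Push is an area-of-effect ability actor, named for a push, that extends a parent class's SpawnAOE event.
; After calling the parent logic, it attaches the NS_Float_ability Niagara system to its root and destroys itself when that system finishes.
; No push logic appears in this Blueprint, and its BeginPlay, overlap and Tick events are disabled stubs.
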(event `self.Spawn AOE`
  (`parent.Spawn AOE`)
  (bind _returnvalue (`NiagaraFunctionLibrary.SpawnSystemAttached` "/Game/test_level/AOE_Asset/AOE_push_Paricle/NS_Float_ability.NS_Float_ability" (`self.DefaultSceneRoot`) "None" (0.0 0.0 0.0) (struct) "KeepRelativeOffset"))
  (add `NiagaraComponent.OnSystemFinished` _returnvalue (delegate `ON_finished`)))

(event `ON_finished`
  (params (PSystem :type "NiagaraComponent Object Reference"))
  (`self.K2_DestroyActor`))

(fn `UserConstructionScript`
  (`parent.UserConstructionScript`))