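; Pickup weapon Blueprint for the classic regular ARMod 5.56 rifle, handling its attachments, magazines and visual effects.
; Construction attaches flashlight and laser parts and delegates procedural recoil and walk setup to BPCWeaponComponent, which also drives scope selection and muzzle smoke.
; SightID selects reticle, offset and FOV correction, with magnified scopes using render-target scene capture while aiming.
; Timelines animate eyepiece spot, suppressor heat glow and raindrop material blending.
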(event `self.Suppressor hot`
  ;[1 1 0] Suppressor Emissive
  (if (== (`.AmmoCurrent_20_1887021F4D4CB2E5D9F559887095BC17` (break `/Game/CGrARModPack/Weapons/Blueprints/PickUp_Master/Gun/BP_WeaponData_Struct` (`self.WeaponData`))) 0)
    _
    (elif (`SceneComponent.IsVisible` (`self.SM_Silencer`))
      (bind (_direction _emissive_alpha) (`Timeline|Timeline_1` :!label _label)
        (:`Update`
          (`MaterialInstanceDynamic.SetScalarParameterValue` (`self.Silencer_DM`) "Emissive Intensity" _emissive_alpha))))))

(event `self.Suppressor cold`
  ;[1 1 0] Suppressor Emissive
  (goto _label :!via `Reverse`))

(event `self.ChamberSmokeActivated`
  ;[1 1 1] ChamberSmokeActivated
  (`ActorComponent.Activate` (`self.ChamberSmoke_PS`) true))

(event `self.ReceiveBeginPlay`
  ;[1 1 0] Suppressor Emissive
  (`parent.ReceiveBeginPlay`)
  (bind _returnvalue (`PrimitiveComponent.CreateDynamicMaterialInstance` (`self.SM_Silencer`) 0 "/Game/CGrARModPack/Weapons/Materials/MaterialInstances/ARMod_Materials/MI_Silencer556_Inst.MI_Silencer556_Inst" "None"))
  (set `self.Silencer_DM` _returnvalue)
  (`SceneComponent.K2_SetRelativeLocation` (`self.MuzzleSmoke_PS`) (0.0 0.0 0.0) false false))

(event `self.SetShadowToComponent_DroppedGun`
  ;[1 1 1] SetShadowToComponents
  (`PrimitiveComponent.SetCastShadow` (`self.Barrel_classic`) true)
  (`PrimitiveComponent.SetCastShadow` (`self.SM_Quadrail_Regular`) true)
  (`PrimitiveComponent.SetCastShadow` (`self.SM_IRSFrame`) true)
  (`PrimitiveComponent.SetCastShadow` (`self.SM_ARMagazine_stl_01`) true))

(event `self.FlashlightAttached`
  ;[1 1 1] FL_attached
  (`self.PicRailCover_Visibility`))

(event `self.SetShadowToComponent_EquippedGun`
  ;[1 1 1] SetShadowToComponents
  (`PrimitiveComponent.SetCastShadow` (`self.Barrel_classic`) false)
  (`PrimitiveComponent.SetCastShadow` (`self.SM_Quadrail_Regular`) false)
  (`PrimitiveComponent.SetCastShadow` (`self.SM_IRSFrame`) false)
  (`PrimitiveComponent.SetCastShadow` (`self.SM_ARMagazine_stl_01`) false))

(event `self.BSmoke_Stop`
  ;[1 1 1] MuzzleSmoke
  (`self.Suppressor hot`)
  (`ActorComponent.Deactivate` (`self.MuzzleSmoke_PS`))
  (`SceneComponent.K2_SetRelativeLocation` (`self.MuzzleSmoke_PS`) (0.0 0.0 0.0) false false))

(event `self.ScopeAttached`
  ;[1 1 1] Scope_attached
  (`/Game/CGrARModPack/Weapons/Blueprints/PickUp_Master/Gun/BPC_WeaponComponent.ScopeSelect` (`self.BPC_WeaponComponent`) (`self.SM_Scope`) (`self.Scopes`) (`self.Sight_ID`))
  (`self.Scope_current`))

(event `self.BSmoke_Start`
  ;[1 1 1] MuzzleSmoke
  (`self.Suppressor cold`)
  (`/Game/CGrARModPack/Weapons/Blueprints/PickUp_Master/Gun/BPC_WeaponComponent.SmokeActivate` (`self.BPC_WeaponComponent`) (`self.WeaponData`) (`self.SM_Silencer`) (`self.MuzzleSmoke_PS`) (20.0 0.0 0.0)))

(event `self.OpGunChek`
  ;[1 1 1] Operative Gun Check
  (`/Game/CGrARModPack/Weapons/Blueprints/PickUp_Master/Gun/BPC_WeaponComponent.OpGunCheck_wSelector` (`self.BPC_WeaponComponent`) (`self.Fire Mode`) (`self.WeaponData`) (`self.Weapon_SKMesh`) 4 "sR_04" "aR_04"))

(event `self.Mag_01_Visible`
  (bind _weapon_skmesh (`self.Weapon_SKMesh`))
  ;[1 1 1] Magazine visibility            (set right materials)
  (`SceneComponent.SetVisibility` (`self.SM_ARMagazine_stl_01`) true false)
  (`PrimitiveComponent.SetMaterialByName` _weapon_skmesh "M_MagFeeder" "/Game/CGrARModPack/Weapons/Materials/MaterialInstances/ARMod_Materials/MI_ARMagazine_stl_Inst.MI_ARMagazine_stl_Inst")
  (`PrimitiveComponent.SetMaterialByName` _weapon_skmesh "M_Cartridge" "/Game/CGrARModPack/Weapons/Materials/MaterialInstances/Some_shared_Materials/MI_556_Cartridge_RGB_Inst.MI_556_Cartridge_RGB_Inst"))

(event `self.MAg_01_Invis`
  (bind _weapon_skmesh (`self.Weapon_SKMesh`))
  ;[1 1 1] Magazine visibility            (set right materials)
  (`SceneComponent.SetVisibility` (`self.SM_ARMagazine_stl_01`) false false)
  (`PrimitiveComponent.SetMaterialByName` _weapon_skmesh "M_MagFeeder" "/Game/CGrARModPack/Weapons/Materials/MasterMaterials/MM_Invisible.MM_Invisible")
  (`PrimitiveComponent.SetMaterialByName` _weapon_skmesh "M_Cartridge" "/Game/CGrARModPack/Weapons/Materials/MasterMaterials/MM_Invisible.MM_Invisible"))

(event `self.eyepiece spot size increase`
  (bind _scene_cc_2d (`self.Scene CC 2D`))
  (bind _eyepiece_spot_size (`self.eyepiece spot size`))
  (bind _sm_scope (`self.SM_Scope`))
  ;[1 1 1] Scope eyepiece spot
  (if (`self.Scope_ID_func`)
    ;[0 1 0] Add scene capture component 2D
    (`self.SetSceneCaptureMaterial`))
  (`/Engine/EditorBlueprintResources/StandardMacros.IsValid` _scene_cc_2d
    (:`Is Valid`
      (`ActorComponent.Activate` _scene_cc_2d false)
      (if (`self.Scope_ID_func`)
        ;;[1 1 1] SetMaterial_ClearGlass
        (`PrimitiveComponent.SetMaterialByName` (`self.SM_Scope`) "M_Glass_B" "/Game/CGrARModPack/Weapons/Materials/MaterialInstances/MI_Glass_Clear_Inst.MI_Glass_Clear_Inst")
        (bind (_direction _newtrack_0) (`Timeline|Timeline_0` :!label _label_2)
          (:`Update`
            (`MaterialInstanceDynamic.SetScalarParameterValue` _eyepiece_spot_size "U_offset" (`KismetMathLibrary.Lerp` (`self.EyepieceSpot_U_offset`) 0.0 _newtrack_0))
            (`MaterialInstanceDynamic.SetScalarParameterValue` _eyepiece_spot_size "V_offset" (`KismetMathLibrary.Lerp` (`self.EyepieceSpot_V_offset`) 0.0 _newtrack_0))))
        (else
          (goto _label_2))))
    (:`Is Not Valid`
      (if (`self.Sight_ID_func`)
        ;[1 1 1] SetMaterial_ClearGlass
        (`PrimitiveComponent.SetMaterialByName` _sm_scope "M_Glass_B" "/Game/CGrARModPack/Weapons/Materials/MaterialInstances/MI_Glass_Clear_Inst.MI_Glass_Clear_Inst")
        (`PrimitiveComponent.SetMaterialByName` _sm_scope "M_Lense_B" "/Game/CGrARModPack/Weapons/Materials/MaterialInstances/MI_Glass_Clear_Inst.MI_Glass_Clear_Inst")))))

(event `self.Mag_02_Vis`
  ;[1 1 1] Magazine visibility            (set right materials)
  (`SceneComponent.SetVisibility` (`self.SM_ARMagazine_stl_02`) true false)
  (`PrimitiveComponent.SetMaterialByName` (`self.Weapon_SKMesh`) "M_Cartridge_inMag02" "/Game/CGrARModPack/Weapons/Materials/MaterialInstances/Some_shared_Materials/MI_556_Cartridge_RGB_Inst.MI_556_Cartridge_RGB_Inst"))

(event `self.eyepiece spot size decrease`
  (bind _scene_cc_2d (`self.Scene CC 2D`))
  (bind _sm_scope (`self.SM_Scope`))
  ;[1 1 1] Scope eyepiece spot
  (`/Engine/EditorBlueprintResources/StandardMacros.IsValid` _scene_cc_2d
    (:`Is Valid`
      (`ActorComponent.Deactivate` _scene_cc_2d)
      (if (`self.Scope_ID_func`)
        ;;[1 1 0] SetMaterial_OpaqueGlass
        (`PrimitiveComponent.SetMaterialByName` (`self.SM_Scope`) "M_Glass_B" "/Game/CGrARModPack/Weapons/Materials/MaterialInstances/MI_OpaqueGlass_Inst.MI_OpaqueGlass_Inst")
        (goto _label_2 :!via `Reverse`)
        (else
          (goto _label_2 :!via `Reverse`))))
    (:`Is Not Valid`
      (if (`self.Sight_ID_func`)
        ;[1 1 0] SetMaterial_OpaqueGlass
        (`PrimitiveComponent.SetMaterialByName` _sm_scope "M_Glass_B" "/Game/CGrARModPack/Weapons/Materials/MaterialInstances/MI_OpaqueGlass_Inst.MI_OpaqueGlass_Inst")
        (`PrimitiveComponent.SetMaterialByName` _sm_scope "M_Lense_B" "/Game/CGrARModPack/Weapons/Materials/MaterialInstances/MI_OpaqueGlass_Inst.MI_OpaqueGlass_Inst")))))

(event `self.Mag_02_invis`
  ;[1 1 1] Magazine visibility            (set right materials)
  (`SceneComponent.SetVisibility` (`self.SM_ARMagazine_stl_02`) false false)
  (`PrimitiveComponent.SetMaterialByName` (`self.Weapon_SKMesh`) "M_Cartridge_inMag02" "/Game/CGrARModPack/Weapons/Materials/MasterMaterials/MM_Invisible.MM_Invisible"))

(event `self.MagEmpty_Invis`
  (bind _weapon_skmesh (`self.Weapon_SKMesh`))
  ;[1 1 1] Magazine visibility            (set right materials)
  (if (<= (`.AmmoCurrent_20_1887021F4D4CB2E5D9F559887095BC17` (break `/Game/CGrARModPack/Weapons/Blueprints/PickUp_Master/Gun/BP_WeaponData_Struct` (`self.WeaponData`))) 1)
    (`PrimitiveComponent.SetMaterialByName` _weapon_skmesh "M_Cartridge" "/Game/CGrARModPack/Weapons/Materials/MasterMaterials/MM_Invisible.MM_Invisible")
    (`PrimitiveComponent.SetMaterialByName` _weapon_skmesh "M_MagFeeder" "/Game/CGrARModPack/Weapons/Materials/MaterialInstances/ARMod_Materials/MI_ARMagazine_stl_Inst.MI_ARMagazine_stl_Inst")))

(event `self.RaindropActivate`
  ;[0.6667 0 0.6517] Raindrops
  ;;[1 1 1] For Reduce the material blend intensity
  (bind (_direction _reduce_the_material_blend_intensity) (`Timeline|Timeline_2` :!label _label_3)
    (:`Update`
      (set `self.Reduce the material blend intensity` _reduce_the_material_blend_intensity)
      (`self.Reduce the material blend intensity_Func`))))

(event `self.RaindropDeactivate`
  ;[0.6667 0 0.6517] Raindrops
  ;;[1 1 1] For Reduce the material blend intensity
  (goto _label_3 :!via `Reverse`))

(event `self.ReceiveTick`
  (params (DeltaSeconds :type "Float (single-precision)"))
  ;[1 1 1] Laser
  (if (not (and (== self (`/Game/CGrARModPack/FPS_Arms/Bluprints/BP_FPS_Arms.CurrentWeapon` (`self.Character Ref`))) (`SceneComponent.IsVisible` (`self.SM_Flashlight`))))
    (`SceneComponent.SetVisibility` (`self.SM_Laser`) false false)
    (`SceneComponent.SetVisibility` (`self.Laser_Point`) false false)
    (else
      (`self.LaserPointPosition`))))

(fn `AddSceneCaptureComponent_func`
  (params (TextureTarget :type "TextureRenderTarget2D Object Reference") (SocketName :type Name) (FOVAngle :type "Float (double-precision)") (`Location correction X` :type "Float (double-precision)"))
  (bind _scene_cc_2d (`self.Scene CC 2D`))
  (bind _returnvalue (`AddComponent|NODE_AddSceneCaptureComponent2D-0`))
  (set `SceneCaptureComponent2D.TextureTarget` TextureTarget _returnvalue)
  (bind _output_get (set `self.Scene CC 2D` _returnvalue))
  (`SceneComponent.K2_AttachToComponent` _output_get (`self.SM_Scope`) SocketName "KeepRelative" "KeepRelative" "KeepRelative" true)
  (set `SceneCaptureComponent2D.FOVAngle` FOVAngle _scene_cc_2d)
  (`SceneComponent.K2_SetRelativeLocation` _scene_cc_2d (`KismetMathLibrary.MakeVector` `Location correction X`) false false))

(fn `AttachToComponent_Func`
  (`SceneComponent.K2_AttachToComponent` (`self.SpotLight`) (`self.SM_Flashlight`) "Light_Sckt" "SnapToTarget" "SnapToTarget" "SnapToTarget" true)
  (`SceneComponent.K2_AttachToComponent` (`self.Laser_Point`) (`self.SM_Flashlight`) "Laser_Sckt" "SnapToTarget" "SnapToTarget" "SnapToTarget" true)
  (`SceneComponent.K2_AttachToComponent` (`self.SM_Laser`) (`self.SM_Flashlight`) "Laser_Sckt" "SnapToTarget" "SnapToTarget" "SnapToTarget" true)
  (`SceneComponent.SetRelativeScale3D` (`self.SM_Laser`) (10.0 0.2 0.2))
  (`SceneComponent.K2_SetRelativeLocation` (`self.SpotLight`) (10.0 0.0 0.0) false false))

(fn `PicRailCover_Visibility`
  (bind _sm_picrail_cover10_top (`self.SM_PicRail_Cover10_Top`))
  (if (`SceneComponent.IsVisible` (`self.SM_Flashlight`))
    (`SceneComponent.SetVisibility` _sm_picrail_cover10_top false false)
    (else
      (`SceneComponent.SetVisibility` _sm_picrail_cover10_top true false))))

(fn `Reduce the material blend intensity_Func`
  ;[1 1 1] Gun body
  (bind _returnvalue (`PrimitiveComponent.CreateDynamicMaterialInstance` (`self.Weapon_SKMesh`) 0 "/Game/CGrARModPack/Weapons/Materials/MaterialInstances/ARMod_Materials/ARMod_MatVariations/MI_ARMod_body_AutumnForestn_Inst.MI_ARMod_body_AutumnForestn_Inst" "None"))
  (`MaterialInstanceDynamic.SetScalarParameterValueByInfo` _returnvalue (`self.LayerMat_BlendIntensity`) (`self.Reduce the material blend intensity`))
  ;[1 1 1] Buttstock
  (bind _returnvalue_2 (`PrimitiveComponent.CreateDynamicMaterialInstance` (`self.Weapon_SKMesh`) 5 "/Game/CGrARModPack/Weapons/Materials/MaterialInstances/Some_shared_Materials/SSM_Variations/MI_ARSStock_AutumnForestn_Inst.MI_ARSStock_AutumnForestn_Inst" "None"))
  (`MaterialInstanceDynamic.SetScalarParameterValueByInfo` _returnvalue_2 (`self.LayerMat_BlendIntensity`) (`self.Reduce the material blend intensity`))
  ;[1 1 1] IRS Frame
  (bind _returnvalue_3 (`PrimitiveComponent.CreateDynamicMaterialInstance` (`self.SM_IRSFrame`) 0 "/Game/CGrARModPack/Weapons/Materials/MaterialInstances/MatVariations/MI_IRSFrame_AutumnForestn_Inst.MI_IRSFrame_AutumnForestn_Inst" "None"))
  (`MaterialInstanceDynamic.SetScalarParameterValueByInfo` _returnvalue_3 (`self.LayerMat_BlendIntensity`) (`self.Reduce the material blend intensity`))
  ;[1 1 1] Buttstock tube
  (`PrimitiveComponent.CreateDynamicMaterialInstance` (`self.Weapon_SKMesh`) 4 "/Game/CGrARModPack/Weapons/Materials/MaterialInstances/Some_shared_Materials/MI_ButtstockTube_Inst.MI_ButtstockTube_Inst" "None")
  ;[1 1 1] PR cover
  (bind _returnvalue_4 (`PrimitiveComponent.CreateDynamicMaterialInstance` (`self.SM_PicRail_Cover10_top`) 0 "/Game/CGrARModPack/Weapons/Materials/MaterialInstances/ARMod_Materials/ARMod_MatVariations/MI_PicRail_Cover_AutumnForestn_Inst.MI_PicRail_Cover_AutumnForestn_Inst" "None"))
  (`MaterialInstanceDynamic.SetScalarParameterValueByInfo` _returnvalue_4 (`self.LayerMat_BlendIntensity`) (`self.Reduce the material blend intensity`))
  (bind _returnvalue_5 (`PrimitiveComponent.CreateDynamicMaterialInstance` (`self.HInstancedSM_SidePicRailCovers`) 0 "/Game/CGrARModPack/Weapons/Materials/MaterialInstances/ARMod_Materials/ARMod_MatVariations/MI_PicRail_Cover_AutumnForestn_Inst.MI_PicRail_Cover_AutumnForestn_Inst" "None"))
  (`MaterialInstanceDynamic.SetScalarParameterValueByInfo` _returnvalue_5 (`self.LayerMat_BlendIntensity`) (`self.Reduce the material blend intensity`))
  (return))

(fn `Scope_current`
  (bind _sm_scope (`self.SM_Scope`))
  (bind _sm_scope_2 (`self.SM_Scope`))
  (bind _sm_irsframe (`self.SM_IRSFrame`))
  (bind _sm_scope_3 (`self.SM_Scope`))
  (bind _sm_scope_4 (`self.SM_Scope`))
  (if (`SceneComponent.IsVisible` (`self.SM_Scope`))
    ;[1 1 1] IRS Frame visibility
    (`SceneComponent.SetVisibility` _sm_irsframe false false)
    (else
      (`SceneComponent.SetVisibility` _sm_irsframe true false)))
  (switch `int` (`self.Sight_ID`)
    (:`0`
      ;[1 1 1] ARDT, RDST and FaLMG HLS location
      (`SceneComponent.K2_SetRelativeLocation` _sm_scope_2 (+ (`SceneComponent.RelativeLocation` _sm_scope_2) (7.0 0.0 0.0)) false false :!label _label))
    (:`1`
      (goto _label))
    (:`2`
      (goto _label))
    (:`4`
      ;[1 1 1] SnpR
      (`|ExecutionSequence`
        (:`then_0`
          ;[1 1 1] Aim Down Sight Field Of View Correction
          (`/Game/CGrARModPack/Weapons/Blueprints/PickUp_Master/Gun/BPC_WeaponComponent.ADS FOV Correction` (`self.BPC_WeaponComponent`) (`self.WeaponData`) -30.0 :!label _label_2))
        (:`then_1`
          ;[1 1 1] SnpR_v1 Scope Retticle
          (`PrimitiveComponent.SetMaterialByName` (`self.SM_Scope`) "M_Layer_2" "/Game/CGrARModPack/Weapons/Materials/MaterialInstances/MI_ParallaxScope_SnpR_RGB_v1.MI_ParallaxScope_SnpR_RGB_v1")
          ;[1 1 1] SnpR Scope
          (`MaterialInstanceDynamic.SetScalarParameterValue` (`self.eyepiece spot size`) "eyepiece spot size" (`self.SnpR_EyepieceSpotSize`) :!label _label_3)
          (`SceneComponent.K2_SetRelativeLocation` _sm_scope (+ (`SceneComponent.RelativeLocation` _sm_scope) (-2.0 0.0 0.0)) false false))))
    (:`7`
      ;[1 1 1] PSO_PR
      (`|ExecutionSequence`
        (:`then_0`
          (goto _label_2))
        (:`then_1`
          (`MaterialInstanceDynamic.SetScalarParameterValue` (`self.eyepiece spot size`) "eyepiece spot size" (`self.PSO_PR_EyepieceSpotSize`))
          (`PrimitiveComponent.SetMaterialByName` (`self.SM_Scope`) "M_Layer_2" "/Game/CGrARModPack/Weapons/Materials/MaterialInstances/MI_ParallaxScope_PSOret_RGB.MI_ParallaxScope_PSOret_RGB")
          (`SceneComponent.K2_SetRelativeLocation` _sm_scope_4 (+ (`SceneComponent.RelativeLocation` _sm_scope_4) (-2.5 0.0 0.0)) false false))))
    (:`9`
      (goto _label))
    (:`10`
      ;[1 1 1] IRS Frame
      (`SceneComponent.K2_SetRelativeLocation` _sm_scope_3 (+ (`SceneComponent.RelativeLocation` _sm_scope_3) (12.13 0.0 0.0)) false false))
    (:`11`
      (goto _label))
    (:`13`
      (`|ExecutionSequence`
        (:`then_0`
          (goto _label_2))
        (:`then_1`
          ;[1 1 1] SnpR_v2 Scope Retticle
          (`PrimitiveComponent.SetMaterialByName` (`self.SM_Scope`) "M_Layer_2" "/Game/CGrARModPack/Weapons/Materials/MaterialInstances/MI_ParallaxScope_SnpR_RGB_v5.MI_ParallaxScope_SnpR_RGB_v5")
          (goto _label_3))))
    (:`14`
      (`|ExecutionSequence`
        (:`then_0`
          (goto _label_2))
        (:`then_1`
          ;[1 1 1] SnpR_v2a Scope Retticle
          (`PrimitiveComponent.SetMaterialByName` (`self.SM_Scope`) "M_Layer_2" "/Game/CGrARModPack/Weapons/Materials/MaterialInstances/MI_ParallaxScope_SnpR_RGB_v2.MI_ParallaxScope_SnpR_RGB_v2")
          (goto _label_3))))
    (:`16`
      ;[1 1 1] SOP \ SOPwR
      (`|ExecutionSequence` :!label _label_4
        (:`then_0`
          (goto _label_2))
        (:`then_1`
          (`PrimitiveComponent.SetMaterialByName` (`self.SM_Scope`) "M_Layer_2" "/Game/CGrARModPack/Weapons/Materials/MaterialInstances/MI_ParallaxScope_PSO2ret_RGB.MI_ParallaxScope_PSO2ret_RGB")
          (`MaterialInstanceDynamic.SetScalarParameterValue` (`self.eyepiece spot size`) "eyepiece spot size" (`self.SOP_PR_EyepieceSpotSize`)))))
    (:`17`
      (goto _label_4))))

(fn `Scope_ID_func`
  (returns (`Correct scopes` :type Boolean))
  (bind _sight_id (`self.Sight_ID`))
  (return (or (== _sight_id 4) (== _sight_id 7) (== _sight_id 13) (== _sight_id 14) (== _sight_id 16) (== _sight_id 17))))

(fn `SetSceneCaptureMaterial`
  ;[1 1 0] SetMaterial RT
  (`PrimitiveComponent.SetMaterialByName` (`self.SM_Scope`) "M_Layer_1" "/Game/CGrARModPack/Weapons/Materials/MaterialInstances/MI_ScopeLayer_01_RT_Inst.MI_ScopeLayer_01_RT_Inst")
  ;[1 0 1] AddSceneCaptureComponent
  (`self.AddSceneCaptureComponent_func` "/Game/CGrARModPack/Weapons/Textures/T_ScopeRT.T_ScopeRT" "Camera_sckt" 3.5 20.0)
  (return))

(fn `Sight_ID_func`
  (returns (`Correct sight` :type Boolean))
  (bind _sight_id (`self.Sight_ID`))
  (return (or (== _sight_id 0) (== _sight_id 8) (== _sight_id 9) (== _sight_id 10))))

(fn `UserConstructionScript`
  (`parent.UserConstructionScript`)
  (`self.AttachToComponent_Func`)
  ;[1 1 1] Variables of Procedural Recoil
  (`/Game/CGrARModPack/Weapons/Blueprints/PickUp_Master/Gun/BPC_WeaponComponent.ProceduralRecoil_func` (`self.BPC_WeaponComponent`) (`self.WeaponData`) (`self.ADSR_PitchMin`) (`self.ADSR_PitchMax`) (`self.ADSR_RollMin`) (`self.ADSR_RollMax`) (`self.ADSR_YawMin`) (`self.ADSR_YawMax`) (`self.ADSR_LocXMin`) (`self.ADSR_LocXMax`) (`self.ADSR_LocYMin`) (`self.ADSR_LocYMax`) (`self.ADSR_LocZMin`) (`self.ADSR_LocZMax`) (`self.R_PitchMin`) (`self.R_PitchMax`) (`self.R_RollMin`) (`self.R_RollMax`) (`self.R_YawMin`) (`self.R_YawMax`) (`self.R_LocXMin`) (`self.R_LocXMax`) (`self.R_LocYMin`) (`self.R_LocYMax`) (`self.R_LocZMin`) (`self.R_LocZMax`) (`self.(Actual)HipFire Recoil Yaw Min`) (`self.(Actual)HipFire Recoil Yaw Max`) (`self.(Actual)HipFire Recoil Pitch Min`) (`self.(Actual)HipFire Recoil Pitch Max`) (`self.(Actual)ADS Recoil Yaw Min`) (`self.(Actual)ADS Recoil Yaw Max`) (`self.(Actual)ADS Recoil Pitch Min`) (`self.(Actual)ADS Recoil Pitch Max`))
  ;[1 1 0] Set Procedural Walk Param
  (`/Game/CGrARModPack/Weapons/Blueprints/PickUp_Master/Gun/BPC_WeaponComponent.ProceduralWalkSet_func` (`self.BPC_WeaponComponent`) 1.0 -1.0 0.5 -0.5 1.0 -1.0 0.5 -0.5 4.0 -4.0 0.7 -0.7)
  (if (or (`self.Scope_ID_func`) (== (`self.Sight_ID`) 0))
    ;[1 1 1] eyepiece spot size
    (bind _returnvalue (`PrimitiveComponent.CreateDynamicMaterialInstance` (`self.SM_Scope`) 4 "/Game/CGrARModPack/Weapons/Materials/MaterialInstances/MI_ScopeLayer_03_Inst.MI_ScopeLayer_03_Inst" "None"))
    (set `self.eyepiece spot size` _returnvalue)))