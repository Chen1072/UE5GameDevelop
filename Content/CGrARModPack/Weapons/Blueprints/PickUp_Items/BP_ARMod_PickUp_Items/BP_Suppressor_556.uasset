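; BP_Suppressor_556 is a pickup item that attaches a 5.56 suppressor to the player's current weapon on interaction.
; It checks the weapon's GunTypeAndCaliber enum against the matching entry and prints a red debug message on a mismatch.
; If the weapon's silencer mesh is hidden, it triggers the player's pickup, waits briefly, plays a sound, shows the mesh, calls SilencerAttached and destroys itself.
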(event `/Game/CGrARModPack/Weapons/Blueprints/PickUp_Master/Interfaces/BPI_Interaction.OnInteracted`
  (params (`Player 0` :type "/Game/CGrARModPack/FPS_Arms/Bluprints/BP_FPS_Arms Object Reference"))
  (bind _currentweapon (`/Game/CGrARModPack/FPS_Arms/Bluprints/BP_FPS_Arms.CurrentWeapon` `Player 0`))
  (bind _sm_silencer (`/Game/CGrARModPack/Weapons/Blueprints/PickUp_Master/Gun/BP_Weapon_Base.SM_Silencer` _currentweapon))
  (`/Engine/EditorBlueprintResources/StandardMacros.IsValid` _currentweapon
    (:`Is Valid`
      (if (`self.Check a Caliber` _currentweapon)
        (if (not (`SceneComponent.IsVisible` _sm_silencer))
          (`/Game/CGrARModPack/FPS_Arms/Bluprints/BP_FPS_Arms.ItemPickUp` `Player 0`)
          (`KismetSystemLibrary.Delay` 0.2)
          (`self.PickUpSound` `Player 0`)
          (`SceneComponent.SetVisibility` _sm_silencer true true)
          (`/Game/CGrARModPack/Weapons/Blueprints/PickUp_Master/Gun/BP_Weapon_Base.SilencerAttached` _currentweapon)
          (`self.K2_DestroyActor`))
        (else
          (`KismetSystemLibrary.PrintString` "the Caliber NOT MATCH" true true (struct :`R` 0.770833 :`A` 1.0)))))))

(fn `Check a Caliber`
  (params (`GunType&Caliber` :type "/Game/CGrARModPack/Weapons/Blueprints/PickUp_Master/Gun/BP_Weapon_Base Object Reference"))
  (returns (` ` :type Boolean))
  ;[0 0 0] Index in "E_GunType_and_Caliber_Enum"
  (return (== (`.GunTypeandCaliber_147_AE58B3FF49A26D3AE1287F8D49F53418` (break `/Game/CGrARModPack/Weapons/Blueprints/PickUp_Master/Gun/BP_WeaponData_Struct` (`/Game/CGrARModPack/Weapons/Blueprints/PickUp_Master/Gun/BP_Weapon_Base.WeaponData` `GunType&Caliber`))) 3)))

(fn `UserConstructionScript`
  (`parent.UserConstructionScript`))