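; Base weapon projectile that deals damage and impact effects on hit, handing itself to player character 0 on BeginPlay through a movement-parameter message.
; A sphere hit sends bone-specific damage to Characters, crediting player 0, and calls SEonCharacter, while other hits call SpawnEmitter.
; Both effect events are empty hooks here.
; Simulating components receive a velocity-scaled impulse, and the projectile destroys itself after a short delay.
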(event `self.ReceiveBeginPlay`
  (message `/Game/CGrARModPack/Weapons/Blueprints/PickUp_Master/Interfaces/BPI_WeaponEventsActivate.ProjectileMovementParam_BPI` (`GameplayStatics.GetPlayerCharacter` 0) self))

(event `self.Sphere.OnComponentHit`
  (params (HitComponent :type "PrimitiveComponent Object Reference") (OtherActor :type "Actor Object Reference") (OtherComp :type "PrimitiveComponent Object Reference") (NormalImpulse :type "Vector Structure") (Hit :type "HitResult Structure (by ref)"))
  (bind (_bblockinghit _binitialoverlap _time _distance _location _impactpoint _normal _impactnormal _physmat _hitactor _hitcomponent _hitbonename) (`GameplayStatics.BreakHitResult` Hit))
  (bind _returnvalue (`KismetMathLibrary.Conv_VectorToRotator` _impactnormal))
  (bind _ascharacter (cast `Character` OtherActor)
    (:`then`
      (message `/Game/CGrARModPack/FPS_Arms/Bluprints/BPI_TakeDamage.TakingDamage` _ascharacter _hitbonename (`self.Damage`) (`GameplayStatics.GetPlayerCharacter` 0))
      (`self.SEonCharacter` _impactpoint _returnvalue))
    (:`CastFailed`
      (`self.SpawnEmitter` _impactpoint _returnvalue _hitcomponent)))
  (if (`SceneComponent.IsSimulatingPhysics` OtherComp "None")
    (`PrimitiveComponent.AddImpulseAtLocation` OtherComp (* (`self.GetVelocity`) (`self.HitImpulse`)) (`self.K2_GetActorLocation`) "None"))
  (`KismetSystemLibrary.Delay` 0.5)
  (`self.K2_DestroyActor`))

(event `SpawnEmitter`
  (params (Location :type "Vector Structure") (Rotation :type "Rotator Structure") (HitComponent :type "PrimitiveComponent Object Reference")))

(event `SEonCharacter`
  (params (Location :type "Vector Structure") (Rotation :type "Rotator Structure") (HitComponent :type "PrimitiveComponent Object Reference")))

(fn `UserConstructionScript`)