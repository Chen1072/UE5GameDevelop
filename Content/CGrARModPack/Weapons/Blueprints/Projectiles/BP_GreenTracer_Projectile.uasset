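; Green tracer bullet projectile Blueprint that supplies the impact effects for world and character hits on top of its parent class.
; SpawnEmitter plays a no-hit and a green hit particle, sets a low hit impulse, and spawns a bullet hole decal actor attached to the hit component.
; SEonCharacter plays a character hit particle and sets a stronger impulse, with no decal.
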(event `self.SpawnEmitter`
  (params (Location :type "Vector Structure") (Rotation :type "Rotator Structure") (HitComponent :type "PrimitiveComponent Object Reference"))
  (`GameplayStatics.SpawnEmitterAtLocation` "/Game/CGrARModPack/DEMO/FX/ParticleSystem/PS_Bullet_NoHit.PS_Bullet_NoHit" Location Rotation (0.35 0.35 0.35))
  (`GameplayStatics.SpawnEmitterAtLocation` "/Game/CGrARModPack/DEMO/FX/ParticleSystem/PS_Bullet_Hit_GreenColor.PS_Bullet_Hit_GreenColor" Location Rotation (0.25 0.25 0.25))
  (set `self.HitImpulse` 0.08)
  (bind _returnvalue (`|SpawnActorFromClass` "/Game/CGrARModPack/Weapons/Blueprints/BP_BulletHoleDecals_Master.BP_BulletHoleDecals_Master_C" (`KismetMathLibrary.MakeTransform` Location Rotation) "Undefined" "OverrideRootScale" null null))
  (`self.K2_AttachToComponent` _returnvalue HitComponent "None" "KeepWorld" "KeepWorld" "KeepWorld" true))

(event `self.SEonCharacter`
  (params (Location :type "Vector Structure") (Rotation :type "Rotator Structure") (HitComponent :type "PrimitiveComponent Object Reference"))
  (`GameplayStatics.SpawnEmitterAtLocation` "/Game/CGrARModPack/DEMO/FX/ParticleSystem/PS_Bullet_HitCharacter.PS_Bullet_HitCharacter" Location Rotation (0.7 0.7 0.7))
  (set `self.HitImpulse` 0.5))

(fn `UserConstructionScript`
  (`parent.UserConstructionScript`))