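; Master hand grenade actor that throws itself along the player's control rotation with random spin, releases its fuse lever, and detonates after a fixed fuse.
; An enum selects frag (radial impulse and falloff damage), stun, or timed smoke, with frag and stun sharing an effects helper.
; Frag and stun blasts at low world Z also spawn an explosion hole and message the player pawn through an interface for hallucination or flashbang effects.
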(event `FuseLever_event`
  (`KismetSystemLibrary.Delay` 0.05)
  (`ActorComponent.Activate` (`self.FuseLever`) false))

(event `self.ReceiveBeginPlay`
  (bind _grenade (`self.Grenade`))
  (bind _returnvalue (`SceneComponent.K2_GetComponentLocation` (`self.Scene`)))
  (bind (_returnvalue_location _returnvalue_rotation) (`KismetMathLibrary.BreakTransform` (`KismetMathLibrary.MakeTransform` (`KismetMathLibrary.MakeVector` (.x _returnvalue) (.y _returnvalue)) (`KismetMathLibrary.MakeRotator` 0.0))))
  (`self.FuseLever_event`)
  (`self.RadialForce_addParam`)
  (`PrimitiveComponent.AddImpulse` _grenade (* (`KismetMathLibrary.GetForwardVector` (`Controller.GetControlRotation` (`GameplayStatics.GetPlayerController` 0))) (800.0 800.0 800.0)) "None" false)
  (`PrimitiveComponent.AddAngularImpulseInDegrees` _grenade (* (`KismetMathLibrary.RandomUnitVector`) 360) "None" false)
  (`KismetSystemLibrary.Delay` 2.0)
  (switch `/Game/CGrARModPack/Weapons/Blueprints/Projectiles/HandGrenades/E_HandGrenade_Enum` (`self.HandGrenadesEnum`)
    (:`NewEnumerator0`
      ;[1 1 1] Frag Grenade
      (`RadialForceComponent.FireImpulse` (`self.RadialForce`))
      (`GameplayStatics.ApplyRadialDamageWithFalloff` :`BaseDamage` 1000.0 :`MinimumDamage` 800.0 :`Origin` (`SceneComponent.K2_GetComponentLocation` (`self.Scene`)) :`DamageInnerRadius` 600.0 :`DamageOuterRadius` 800.0 :`DamageFalloff` 1.0 :`DamageCauser` (`GameplayStatics.GetPlayerCharacter` 0) :`InstigatedByController` null :`DamagePreventionChannel` "ECC_GameTraceChannel4")
      (bind _outputpin (`self.ExplosionEmitters_func` "/Game/CGrARModPack/Weapons/Audio/SC_ExplosionGLGrensde_Cue.SC_ExplosionGLGrensde_Cue" "/Game/CGrARModPack/DEMO/FX/ParticleSystem/PS_Bullet_NoHit.PS_Bullet_NoHit" "/Game/CGrARModPack/DEMO/FX/ParticleSystem/PS_Bullet_Hit_YellowColor.PS_Bullet_Hit_YellowColor" "/Game/CGrARModPack/DEMO/FX/ParticleSystem/P_Explosion_FragGrenade.P_Explosion_FragGrenade"))
      (if (<= (.z _outputpin) 50.0)
        (bind _returnvalue_2 (`|SpawnActorFromClass` "/Game/CGrARModPack/Weapons/Blueprints/BP_ExplHole_Child.BP_ExplHole_Child_C" (`KismetMathLibrary.MakeTransform` (`KismetMathLibrary.MakeVector` (.x _outputpin) (.y _outputpin)) (`KismetMathLibrary.MakeRotator` 0.0 90.0) (20.0 20.0 20.0)) "Undefined" "OverrideRootScale" null null))
        (`self.K2_AttachToComponent` _returnvalue_2 null "None" "KeepWorld" "KeepWorld" "KeepWorld" true)
        ;;[1 1 1] Interface Masage
        (message `/Game/CGrARModPack/Weapons/Blueprints/PickUp_Master/Interfaces/BPI_WeaponEventsActivate.FragGrenadeHallusion_BPI` (`GameplayStatics.GetPlayerPawn` 0) (`KismetMathLibrary.Vector_Distance` (`self.K2_GetActorLocation` (`GameplayStatics.GetPlayerPawn` 0)) (`self.K2_GetActorLocation`)) (`SceneComponent.K2_GetComponentLocation` (`self.Scene`)))
        (`self.K2_DestroyActor` self)
        (else
          (`self.K2_DestroyActor` self))))
    (:`NewEnumerator1`
      ;[1 1 1] Stun Grenade
      (bind _outputpin_2 (`self.ExplosionEmitters_func` "/Game/CGrARModPack/Weapons/Audio/SC_StunGrenade_Cue.SC_StunGrenade_Cue" "/Game/CGrARModPack/DEMO/FX/ParticleSystem/PS_Bullet_NoHit.PS_Bullet_NoHit" "/Game/CGrARModPack/DEMO/FX/ParticleSystem/PS_Bullet_Hit_YellowColor.PS_Bullet_Hit_YellowColor" "/Game/CGrARModPack/DEMO/FX/ParticleSystem/P_StunGrenade.P_StunGrenade"))
      (if (<= (.z _outputpin_2) 50.0)
        (bind _returnvalue_3 (`|SpawnActorFromClass` "/Game/CGrARModPack/Weapons/Blueprints/BP_ExplHoleSG_Child.BP_ExplHoleSG_Child_C" (`KismetMathLibrary.MakeTransform` (`KismetMathLibrary.MakeVector` (.x _outputpin_2) (.y _outputpin_2)) (`KismetMathLibrary.MakeRotator` 0.0 90.0) (2.0 20.0 20.0)) "Undefined" "OverrideRootScale" null null))
        (`self.K2_AttachToComponent` _returnvalue_3 null "None" "KeepWorld" "KeepWorld" "KeepWorld" true)
        ;[1 1 1] Interface Masage
        (message `/Game/CGrARModPack/Weapons/Blueprints/PickUp_Master/Interfaces/BPI_WeaponEventsActivate.FlashBang_BPI` (`GameplayStatics.GetPlayerPawn` 0) (`KismetMathLibrary.Vector_Distance` (`self.K2_GetActorLocation` (`GameplayStatics.GetPlayerPawn` 0)) (`self.K2_GetActorLocation`)) (`SceneComponent.K2_GetComponentLocation` (`self.Scene`)))
        (`self.K2_DestroyActor` self)
        (else
          (`self.K2_DestroyActor` self))))
    (:`NewEnumerator2`
      ;[1 1 1] Smoke Grenade
      (`GameplayStatics.PlaySoundAtLocation` "/Game/CGrARModPack/Weapons/Audio/SC_SmokeGrenade_Cue.SC_SmokeGrenade_Cue" _returnvalue (struct) 1.0 1.0 0.0 null null null)
      (bind _returnvalue_4 (`GameplayStatics.SpawnEmitterAtLocation` "/Game/CGrARModPack/DEMO/FX/ParticleSystem/P_SmokeGrenade.P_SmokeGrenade" _returnvalue_location _returnvalue_rotation (3.0 3.0 3.0)))
      (`KismetSystemLibrary.Delay` 14.0)
      (`ActorComponent.Deactivate` _returnvalue_4)
      (`self.K2_DestroyActor` self))))

(fn `ExplosionEmitters_func`
  (params (Sound :type "SoundBase Object Reference") (EmitterTemplate01 :type "ParticleSystem Object Reference") (EmitterTemplate02 :type "ParticleSystem Object Reference") (EmitterTemplate03 :type "ParticleSystem Object Reference"))
  (returns (OutputPin :type "Vector Structure"))
  (bind _scene (`self.Scene`))
  (bind _returnvalue (`SceneComponent.K2_GetComponentLocation` _scene))
  (bind _returnvalue_2 (`SceneComponent.K2_GetComponentRotation` _scene))
  (`GameplayStatics.PlaySoundAtLocation` Sound _returnvalue (struct) 1.0 1.0 0.0 null null null)
  (`GameplayStatics.SpawnEmitterAtLocation` EmitterTemplate01 _returnvalue _returnvalue_2 (3.0 3.0 3.0))
  (`GameplayStatics.SpawnEmitterAtLocation` EmitterTemplate02 _returnvalue _returnvalue_2 (5.0 5.0 5.0))
  (`GameplayStatics.SpawnEmitterAtLocation` EmitterTemplate03 _returnvalue _returnvalue_2)
  (return _returnvalue))

(fn `RadialForce_addParam`
  (bind _radialforce (`self.RadialForce`))
  (`RadialForceComponent.AddObjectTypeToAffect` _radialforce "ObjectTypeQuery10")
  (`RadialForceComponent.AddObjectTypeToAffect` _radialforce "ObjectTypeQuery9")
  (set `RadialForceComponent.Radius` 700.0 _radialforce)
  (set `RadialForceComponent.bImpulseVelChange` true _radialforce)
  (set `RadialForceComponent.ForceStrength` 1500.0 _radialforce))

(fn `UserConstructionScript`)