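; Interactable ammo box pickup that refills the reserve ammo (AmmoMax) of the player's current weapon up to that weapon's PickUpAmmoPool.
; On interaction it shows the magazine, prints "Full Ammo" if the reserve equals the pool, or plays pickup sounds, updates the reserve and auto-reloads an empty weapon.
; Open and close events set the player's PickUpItemOpened flag and pass it to the box's anim instance through BoxMessage.
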(event `/Game/CGrARModPack/Weapons/Blueprints/PickUp_Master/Interfaces/BPI_Interaction.OnInteracted`
  (params (`Player 0` :type "/Game/CGrARModPack/FPS_Arms/Bluprints/BP_FPS_Arms Object Reference"))
  (bind _currentweapon (`/Game/CGrARModPack/FPS_Arms/Bluprints/BP_FPS_Arms.CurrentWeapon` `Player 0`))
  (bind _currentweapon_2 (`/Game/CGrARModPack/FPS_Arms/Bluprints/BP_FPS_Arms.CurrentWeapon` `Player 0`))
  (bind _weapondata (`/Game/CGrARModPack/Weapons/Blueprints/PickUp_Master/Gun/BP_Weapon_Base.WeaponData` _currentweapon_2))
  (bind ((`AmmoMax_16_07E5E6CD4099A151EC845390F8F05DD9` _ammomax) (`PickUp_AmmoPool_153_D0047CFE4D1648399ACE53B72548269D` _pickup_ammopool)) (break `/Game/CGrARModPack/Weapons/Blueprints/PickUp_Master/Gun/BP_WeaponData_Struct` (`/Game/CGrARModPack/Weapons/Blueprints/PickUp_Master/Gun/BP_Weapon_Base.WeaponData` _currentweapon)))
  (bind _returnvalue (+ (`self.PickUpAmmo`) _ammomax))
  (`/Engine/EditorBlueprintResources/StandardMacros.IsValid` _currentweapon
    (:`Is Valid`
      (`/Game/CGrARModPack/Weapons/Blueprints/PickUp_Master/Gun/BP_Weapon_Base.MagVisible` _currentweapon)
      (set `self.PickupAmmo` _pickup_ammopool)
      (if (== _ammomax (`self.PickUpAmmo`))
        (`KismetSystemLibrary.PrintString` "Full Ammo" true true (struct :`G` 0.2 :`B` 1.0 :`A` 1.0))
        (else
          (`self.PickUpSound` `Player 0`)
          (`self.AmmoPickUpSound` `Player 0`)
          (if (>= _returnvalue (`self.PickUpAmmo`))
            (setmembers `/Game/CGrARModPack/Weapons/Blueprints/PickUp_Master/Gun/BP_WeaponData_Struct` :`StructRef` _weapondata :`Ammo Max` (`self.PickUpAmmo`))
            (if (== (`.AmmoCurrent_20_1887021F4D4CB2E5D9F559887095BC17` (break `/Game/CGrARModPack/Weapons/Blueprints/PickUp_Master/Gun/BP_WeaponData_Struct` _weapondata)) 0)
              (`/Game/CGrARModPack/Weapons/Blueprints/PickUp_Master/Gun/BP_Weapon_Base.AutoReload` _currentweapon_2))
            (else
              (setmembers `/Game/CGrARModPack/Weapons/Blueprints/PickUp_Master/Gun/BP_WeaponData_Struct` :`StructRef` _weapondata :`Ammo Max` _returnvalue))))))))

(event `self.Item_AnimOpen`
  ;[1 1 1] Open Box variable
  (bind _output_get (set `/Game/CGrARModPack/FPS_Arms/Bluprints/BP_FPS_Arms.PickUpItem_Opened` true (`self.PlayerRef`)))
  (message `/Game/CGrARModPack/Weapons/Blueprints/PickUp_Master/Interfaces/BPI_Box.Box` (`SkeletalMeshComponent.GetAnimInstance` (`self.SKM_Box_Ammo`)) _output_get))

(event `self.Item_AnimClose`
  ;[1 1 1] Open Box variable
  (bind _output_get (set `/Game/CGrARModPack/FPS_Arms/Bluprints/BP_FPS_Arms.PickUpItem_Opened` false (`self.PlayerRef`)))
  (message `/Game/CGrARModPack/Weapons/Blueprints/PickUp_Master/Interfaces/BPI_Box.Box` (`SkeletalMeshComponent.GetAnimInstance` (`self.SKM_Box_Ammo`)) _output_get))

(fn `AmmoPickUpSound`
  (params (Out_Player :type "/Game/CGrARModPack/FPS_Arms/Bluprints/BP_FPS_Arms Object Reference"))
  (`GameplayStatics.PlaySoundAtLocation` "/Game/CGrARModPack/Weapons/Audio/SC_Mag_insert_Empty_Cue.SC_Mag_insert_Empty_Cue" (`SceneComponent.K2_GetComponentLocation` (`/Game/CGrARModPack/FPS_Arms/Bluprints/BP_FPS_Arms.Arms` Out_Player)) (struct) 1.0 1.0 0.0 null null null)
  (return))

(fn `UserConstructionScript`
  (`parent.UserConstructionScript`))