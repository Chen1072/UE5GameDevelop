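; Base area-of-effect actor that runs a one-shot sphere overlap at its location on BeginPlay.
; SpawnAOE draws a debug sphere, then queries a single object type within a fixed radius, ignoring the instigator.
; Each hit actor is passed to the AOEOverlapActor dispatcher call and its name is printed, leaving the actual effect outside this graph.
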(event `self.ReceiveBeginPlay`
  (`self.Spawn AOE`))

(event `Spawn AOE`
  (bind _returnvalue (`self.K2_GetActorLocation`))
  (bind _radius (`self.Radius`))
  (set `self.Radius` 450.0)
  (`KismetSystemLibrary.DrawDebugSphere` _returnvalue _radius 12 (struct :`R` 1.0 :`G` 1.0 :`B` 1.0 :`A` 1.0) 2.0)
  (bind _outactors (`KismetSystemLibrary.SphereOverlapActors` _returnvalue _radius (`|MakeArray` "ObjectTypeQuery10" :!type "EObjectTypeQuery Enum") null (`|MakeArray` (`self.GetInstigator`) :!type "Actor Object Reference")))
  (for _array_element _outactors
    (`self.AOEOverlapActor` _array_element)
    (`KismetSystemLibrary.PrintString` (`KismetSystemLibrary.GetDisplayName` _array_element))))

(fn `UserConstructionScript`)