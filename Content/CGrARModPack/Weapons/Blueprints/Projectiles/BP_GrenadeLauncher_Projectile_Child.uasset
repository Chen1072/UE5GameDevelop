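; Grenade launcher projectile, a child Blueprint that explodes on impact with radial damage and physics impulse.
; BeginPlay tunes projectile movement and configures the inherited RadialForce.
; SpawnEmitter handles surface hits with explosion effects and an attached explosion hole, while SEonCharacter plays character-hit effects with a far higher HitImpulse.
; Both fire the impulse, apply falloff damage credited to player 0, play sound and send that pawn a distance-based FragGrenadeHallusion interface message.
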(event `self.ReceiveBeginPlay`
  (bind _projectilemovement (`self.ProjectileMovement`))
  (`parent.ReceiveBeginPlay`)
  (set `ProjectileMovementComponent.ProjectileGravityScale` 2.0 _projectilemovement)
  (set `ProjectileMovementComponent.InitialSpeed` 7000.0 _projectilemovement)
  (set `ProjectileMovementComponent.MaxSpeed` 8000.0 _projectilemovement)
  (`self.RadialForce_addParam`))

(event `self.SpawnEmitter`
  (params (Location :type "Vector Structure") (Rotation :type "Rotator Structure") (HitComponent :type "PrimitiveComponent Object Reference"))
  (bind _radialforce (`self.RadialForce`))
  (`GameplayStatics.SpawnEmitterAtLocation` "/Game/CGrARModPack/DEMO/FX/ParticleSystem/PS_Bullet_NoHit.PS_Bullet_NoHit" Location Rotation (3.0 3.0 3.0))
  (`GameplayStatics.SpawnEmitterAtLocation` "/Game/CGrARModPack/DEMO/FX/ParticleSystem/PS_Bullet_Hit_YellowColor.PS_Bullet_Hit_YellowColor" Location Rotation (5.0 5.0 5.0))
  (`GameplayStatics.SpawnEmitterAtLocation` "/Game/CGrARModPack/DEMO/FX/ParticleSystem/P_Explosion_GrenadeLauncher.P_Explosion_GrenadeLauncher" Location Rotation)
  (set `self.HitImpulse` 10.0)
  (bind _returnvalue (`|SpawnActorFromClass` "/Game/CGrARModPack/Weapons/Blueprints/BP_ExplHole_Child.BP_ExplHole_Child_C" (`KismetMathLibrary.MakeTransform` Location Rotation (20.0 20.0 20.0)) "Undefined" "OverrideRootScale" null null))
  (`self.K2_AttachToComponent` _returnvalue HitComponent "None" "KeepWorld" "KeepWorld" "KeepWorld" true)
  (`ActorComponent.Activate` _radialforce false)
  (`RadialForceComponent.FireImpulse` _radialforce)
  (`GameplayStatics.ApplyRadialDamageWithFalloff` :`BaseDamage` 500.0 :`MinimumDamage` 100.0 :`Origin` (+ Location (0.0 0.0 200.0)) :`DamageInnerRadius` 400.0 :`DamageOuterRadius` 600.0 :`DamageFalloff` 1.0 :`DamageCauser` (`GameplayStatics.GetPlayerCharacter` 0) :`InstigatedByController` null :`DamagePreventionChannel` "ECC_GameTraceChannel4")
  (`GameplayStatics.PlaySoundAtLocation` "/Game/CGrARModPack/Weapons/Audio/SC_ExplosionGLGrensde_Cue.SC_ExplosionGLGrensde_Cue" Location (struct) 1.0 1.0 0.0 null null null)
  ;[1 1 1] Interface Masage
  (message `/Game/CGrARModPack/Weapons/Blueprints/PickUp_Master/Interfaces/BPI_WeaponEventsActivate.FragGrenadeHallusion_BPI` (`GameplayStatics.GetPlayerPawn` 0) (`KismetMathLibrary.Vector_Distance` (`self.K2_GetActorLocation` (`GameplayStatics.GetPlayerPawn` 0)) (`self.K2_GetActorLocation`)) Location))

(event `self.SEonCharacter`
  (params (Location :type "Vector Structure") (Rotation :type "Rotator Structure") (HitComponent :type "PrimitiveComponent Object Reference"))
  (bind _radialforce (`self.RadialForce`))
  (`GameplayStatics.SpawnEmitterAtLocation` "/Game/CGrARModPack/DEMO/FX/ParticleSystem/PS_Bullet_HitCharacter.PS_Bullet_HitCharacter" Location Rotation)
  (`GameplayStatics.SpawnEmitterAtLocation` "/Game/CGrARModPack/DEMO/FX/ParticleSystem/PS_Bullet_Hit_YellowColor.PS_Bullet_Hit_YellowColor" Location Rotation (2.0 2.0 2.0))
  (set `self.HitImpulse` 20000.0)
  (`ActorComponent.Activate` _radialforce false)
  (`RadialForceComponent.FireImpulse` _radialforce)
  (`GameplayStatics.ApplyRadialDamageWithFalloff` :`BaseDamage` 500.0 :`MinimumDamage` 100.0 :`Origin` Location :`DamageInnerRadius` 400.0 :`DamageOuterRadius` 600.0 :`DamageFalloff` 1.0 :`DamageCauser` (`GameplayStatics.GetPlayerCharacter` 0) :`InstigatedByController` null :`DamagePreventionChannel` "ECC_GameTraceChannel4")
  (`GameplayStatics.PlaySoundAtLocation` "/Game/CGrARModPack/Weapons/Audio/SC_ExplosionGLGrensde_Cue.SC_ExplosionGLGrensde_Cue" Location (struct) 1.0 1.0 0.0 null null null)
  ;[1 1 1] Interface Masage
  (message `/Game/CGrARModPack/Weapons/Blueprints/PickUp_Master/Interfaces/BPI_WeaponEventsActivate.FragGrenadeHallusion_BPI` (`GameplayStatics.GetPlayerPawn` 0) (`KismetMathLibrary.Vector_Distance` (`self.K2_GetActorLocation` (`GameplayStatics.GetPlayerPawn` 0)) (`self.K2_GetActorLocation`)) Location))

(fn `RadialForce_addParam`
  (bind _radialforce (`self.RadialForce`))
  (`RadialForceComponent.AddObjectTypeToAffect` _radialforce "ObjectTypeQuery10")
  (`RadialForceComponent.AddObjectTypeToAffect` _radialforce "ObjectTypeQuery9")
  (set `RadialForceComponent.Radius` 400.0 _radialforce)
  (set `RadialForceComponent.bImpulseVelChange` true _radialforce)
  (set `RadialForceComponent.ForceStrength` 1000.0 _radialforce)
  (return))

(fn `UserConstructionScript`
  (`parent.UserConstructionScript`))