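; Base pickup Blueprint that shows an on-screen interaction prompt while a player is in interaction range.
; Range entry stores the player, creates a screen-space widget component at an attach point and calls the open-animation hook; exit destroys it and calls the close hook.
; Prompt text and attach point come from functions defaulting to "Interact" and the scene root.
; Interaction and animation events are empty stubs, and a helper plays the pickup sound at the player's arms.
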(event `/Game/CGrARModPack/Weapons/Blueprints/PickUp_Master/Interfaces/BPI_Interaction.OnInteractionRnageEntered`
  (params (`Player 0` :type "/Game/CGrARModPack/FPS_Arms/Bluprints/BP_FPS_Arms Object Reference"))
  (set `self.PlayerRef` `Player 0`)
  (`self.InteractionWidgetComponent`
    (:`then`)
    (:`else`
      (bind _returnvalue (`|CreateWidget` "/Game/CGrARModPack/Weapons/Blueprints/PickUp_Master/WB_InteractionWidget.WB_InteractionWidget_C" (cast `PlayerController` (`Pawn.GetController` `Player 0`) :!pure true) (`self.Get Interaction Text`)))
      (bind _returnvalue_2 (`AddComponent|NODE_AddWidgetComponent-0`))
      (bind _output_get (set `self.InteractionWidgetComponent` _returnvalue_2))
      (`WidgetComponent.SetWidget` _output_get _returnvalue)
      (`WidgetComponent.SetWidgetSpace` _output_get "Screen")
      (`WidgetComponent.SetDrawAtDesiredSize` _output_get true)
      (`PrimitiveComponent.SetCollisionEnabled` _output_get "NoCollision")
      (`SceneComponent.K2_AttachToComponent` _output_get (`self.Get Interaction Text Attach`) "None" "SnapToTarget" "SnapToTarget" "SnapToTarget" true)
      (`self.Item_AnimOpen`))))

(event `/Game/CGrARModPack/Weapons/Blueprints/PickUp_Master/Interfaces/BPI_Interaction.OnInteractionRnageExited`
  (bind _interactionwidgetcomponent (`self.InteractionWidgetComponent`)
    (:`then`
      (`ActorComponent.K2_DestroyComponent` _interactionwidgetcomponent)
      (`self.Item_AnimClose`))
    (:`else`)))

(event `Item_AnimOpen`)

(event `Item_AnimClose`)

(event `/Game/CGrARModPack/Weapons/Blueprints/PickUp_Master/Interfaces/BPI_Interaction.OnInteracted`
  (params (`Player 0` :type "/Game/CGrARModPack/FPS_Arms/Bluprints/BP_FPS_Arms Object Reference")))

(fn `Get Interaction Text`
  (returns (text :type Text))
  (return "Interact"))

(fn `Get Interaction Text Attach`
  (returns (DefaultSceneRoot :type "SceneComponent Object Reference"))
  (return (`self.DefaultSceneRoot`)))

(fn `PickUpSound`
  (params (Out_Player :type "/Game/CGrARModPack/FPS_Arms/Bluprints/BP_FPS_Arms Object Reference"))
  (`GameplayStatics.PlaySoundAtLocation` "/Game/CGrARModPack/FPS_Arms/Audio/SC_PickUp_Cue.SC_PickUp_Cue" (`SceneComponent.K2_GetComponentLocation` (`/Game/CGrARModPack/FPS_Arms/Bluprints/BP_FPS_Arms.Arms` Out_Player)) (struct) 1.0 1.0 0.0 null null null)
  (return))

(fn `UserConstructionScript`)